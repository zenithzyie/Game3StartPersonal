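; BP_Coing is a collectible coin actor that the player picks up by pressing E.
; Character overlap enables input; E increments the character's ScoreCoing, calls DidYouWin, plays a sound at world origin and destroys the coin.
; LoadCollectedState applies a pink emissive material and clears CanCollect.
; The CanCollect check and both save-recording branches, via game mode and game instance, are disconnected.
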(event OnComponentBeginOverlap(StaticMesh)
  (params (OverlappedComponent :type Primitive%20Component%20Object%20Reference) (OtherActor :type Actor%20Object%20Reference) (OtherComp :type Primitive%20Component%20Object%20Reference) (OtherBodyIndex :type Integer) (bFromSweep :type Boolean) (SweepResult :type Hit%20Result%20Structure%20%28by%20ref%29))
  (bind _asbp_third_person_character (Utilities|Casting|CastToBP_ThirdPersonCharacter OtherActor))
  (Input|EnableInput (Game|GetPlayerController 0)))

(event Custom|LoadCollectedState
  (Rendering|Material|SetMaterial (Variables|Default|GetStaticMesh) 0 "/Game/Materials/MI_EmissivePink.MI_EmissivePink")
  (Variables|Default|SetCanCollect false)
  (Development|PrintString "Collected State loaded"))

(event Input|KeyboardEvents|E
  (params (Key :type Key%20Structure :default "None"))
  (:Pressed
    (Variables|/Game/ThirdPerson/Blueprints/BP_ThirdPersonCharacter.BP_ThirdPersonCharacter_C|SetScoreCoing (stale OnComponentBeginOverlap(StaticMesh) _asbp_third_person_character) (+ (Variables|/Game/ThirdPerson/Blueprints/BP_ThirdPersonCharacter.BP_ThirdPersonCharacter_C|GetScoreCoing (stale OnComponentBeginOverlap(StaticMesh) _asbp_third_person_character)) 1))
    (Default|DidYouWin (stale OnComponentBeginOverlap(StaticMesh) _asbp_third_person_character))
    (Audio|PlaySoundatLocation "/Game/Audio/DirtSteps/dirt_step-001.dirt_step-001" "0, 0, 0" "0, 0, 0" 1.0 1.0 0.0 0 0 0 0)
    (Actor|DestroyActor)))

(fn ConstructionScript)