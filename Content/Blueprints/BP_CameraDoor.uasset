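; BP_CameraDoor is a door meant to show its opening through a temporary camera cutscene.
; Its sequence blends the view to the door actor, lowers the Door component with a Timeline lerp, waits, then blends back to NewViewTarget, the player, in half the time.
; That sequence is currently disconnected: OpenDoor only checks Closed and does nothing.
; A stray, unwired GameMode-to-character cast with AddUnique also remains.
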(event Custom|OpenDoor
  (params (NewViewTarget :type Actor%20Object%20Reference))
  (if (Variables|Default|GetClosed)
    _))

(fn ConstructionScript)