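; BP_Piston is an animated piston actor that moves up and down with a thud sound.
; On BeginPlay a timeline drives the Piston component's relative Z, and its Thud event plays an attenuated sound at the piston's location.
; The timeline's new-time input takes a random float, apparently to stagger instances.
; Force feedback and camera shake nodes are present but never run.
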(event EventBeginPlay
  (Utilities|FlowControl|Sequence
    (:then_0
      (bind _newtrack_0 (Timeline|Timeline Play)
        (:Update
          (Transformation|SetRelativeLocation (Variables|Default|GetPiston) (Math|Vector|MakeVector 0.0 0.0 (- (* _newtrack_0 4e+01) 2e+01)) false false))
        (:Thud
          (Audio|SpawnSoundatLocation "/Game/Audio/HitHurt5OneShot.HitHurt5OneShot" (Transformation|GetWorldLocation (Variables|Default|GetPiston)) "0, 0, 0" 1.0 1.0 0.0 "/Game/Audio/ATT_DefaultAttenuation.ATT_DefaultAttenuation" 0))))
    (:then_1
      (Timeline|Timeline SetNewTime))))

(fn ConstructionScript)