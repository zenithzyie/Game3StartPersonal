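; BP_Deckard is a speaking character that plays a dialogue wave at its location when certain actors enter its Sphere.
; The overlap event casts the other actor in turn to Booperson, Greenie, then the third-person character, ignoring anything else.
; Each match builds a dialogue context from Deckard's voice and that actor's voice, so one wave can vary by listener.
; The player match also prints a greeting.
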(event OnComponentBeginOverlap(Sphere)
  (params (OverlappedComponent :type Primitive%20Component%20Object%20Reference) (OtherActor :type Actor%20Object%20Reference) (OtherComp :type Primitive%20Component%20Object%20Reference) (OtherBodyIndex :type Integer) (bFromSweep :type Boolean) (SweepResult :type Hit%20Result%20Structure%20%28by%20ref%29))
  (bind _returnvalue (Transformation|GetActorLocation))
  (bind _voice (Variables|Default|GetVoice))
  ;[1 1 1] Comment
  (bind _asbp_booperson (Utilities|Casting|CastToBP_Booperson OtherActor)
    (:then
      (Class|GameplayStatics|PlayDialogueatLocation (Variables|Default|GetWave) (Utilities|Struct|MakeDialogueContext _voice (Utilities|Array|MakeArray (Variables|/Game/Old_Dialogue/BP_Booperson.BP_Booperson_C|GetVoice _asbp_booperson))) _returnvalue "0, 0, 0" 1.0 1.0 0.0 0))
    (:CastFailed
      (bind _asbp_greenie (Utilities|Casting|CastToBP_Greenie OtherActor)
        (:then
          (Class|GameplayStatics|PlayDialogueatLocation (Variables|Default|GetWave) (Utilities|Struct|MakeDialogueContext _voice (Utilities|Array|MakeArray (Variables|/Game/Old_Dialogue/BP_Greenie.BP_Greenie_C|GetVoice _asbp_greenie))) _returnvalue "0, 0, 0" 1.0 1.0 0.0 0))
        (:CastFailed
          (bind _asbp_third_person_character (Utilities|Casting|CastToBP_ThirdPersonCharacter OtherActor))
          (Class|GameplayStatics|PlayDialogueatLocation (Variables|Default|GetWave) (Utilities|Struct|MakeDialogueContext (Variables|Default|GetVoice) (Utilities|Array|MakeArray (Variables|/Game/ThirdPerson/Blueprints/BP_ThirdPersonCharacter.BP_ThirdPersonCharacter_C|GetDialogueVoice _asbp_third_person_character))) _returnvalue "0, 0, 0" 1.0 1.0 0.0 0)
          (Development|PrintString "Hello player"))))))

(fn ConstructionScript)