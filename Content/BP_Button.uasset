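; BP_Button is a pressable button actor that animates and plays a click sound on the ClickButton input action.
; Any overlap with its Sphere enables player input on the actor, with no matching disable.
; BeginPlay caches the raised and lowered relative transforms of the Button component.
; On press, the ButtonIn timeline lerps it down, then ButtonOut, played in reverse, lerps it back up.
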(event OnComponentBeginOverlap(Sphere)
  (params (OverlappedComponent :type Primitive%20Component%20Object%20Reference) (OtherActor :type Actor%20Object%20Reference) (OtherComp :type Primitive%20Component%20Object%20Reference) (OtherBodyIndex :type Integer) (bFromSweep :type Boolean) (SweepResult :type Hit%20Result%20Structure%20%28by%20ref%29))
  (Input|EnableInput (Game|GetPlayerController 0)))

(event EventBeginPlay
  (bind _button (Variables|Default|GetButton))
  (bind _returnvalue (Transformation|GetRelativeTransform _button))
  (Variables|Default|SetOutPos (Math|Transform|MakeTransform (.location _returnvalue) (.rotation _returnvalue) (.scale _returnvalue)))
  (Variables|Default|SetInPos (Math|Transform|MakeTransform (- (.location _returnvalue) "0.000000,0.000000,10.000000") (.rotation _returnvalue) (.scale _returnvalue))))

(event Input|ActionEvents|InputActionClickButton
  (params (Key :type Key%20Structure :default "None"))
  (:Pressed
    (Development|PrintString "CLICKEDBUTTON")
    (Audio|PlaySoundatLocation "/Game/ButtonClickSound.ButtonClickSound" (Transformation|GetActorLocation (Game|GetPlayerCharacter 0)) "0, 0, 0" 1.0 1.0 0.0 0 0 0 0)
    (bind _buttonin (Timeline|ButtonIn PlayFromStart)
      (:Update
        (Transformation|SetRelativeTransform (Variables|Default|GetButton) (Math|Transform|Lerp(Transform) (Variables|Default|GetOutPos) (Variables|Default|GetInPos) _buttonin) false false))
      (:Finished
        (bind _buttonin_2 (Timeline|ButtonOut ReverseFromEnd)
          (:Update
            (Transformation|SetRelativeTransform (Variables|Default|GetButton) (Math|Transform|Lerp(Transform) (Variables|Default|GetOutPos) (Variables|Default|GetInPos) _buttonin_2) false false)))))))

(fn ConstructionScript)