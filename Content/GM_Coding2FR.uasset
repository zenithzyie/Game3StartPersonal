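; Game mode for Coding2FR that sets up per-level save data when play begins, using the current level name as the save slot.
; An existing slot is loaded as SG_LevelSave, which runs its LevelCollectedCoins call and moves the player to the saved transform unless that location is zero.
; Without a slot, it creates a new save object in memory and keeps it in LevelSave, without writing it to disk.
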(event EventBeginPlay
  ;[1 1 1] Is there level save for this level's name? If no - create one so we can edit it.
  (Development|PrintString "Loaded into the Coding2FR Gamemode" true true "(R=0.886818,G=0.491155,B=1.000000,A=1.000000)" 2e+01)
  (bind _returnvalue (Game|GetCurrentLevelName true))
  (bind _returnvalue_2 (SaveGame|DoesSaveGameExist _returnvalue))
  (if _returnvalue_2
    (bind _returnvalue_3 (SaveGame|LoadGamefromSlot _returnvalue))
    (bind _assg_level_save (Utilities|Casting|CastToSG_LevelSave _returnvalue_3))
    (bind _output_get (Variables|Default|SetLevelSave _assg_level_save))
    (Default|LevelCollectedCoins _output_get)
    (if (not (Class|KismetMathLibrary|EqualExactlyVectorVector (.location (Variables|/Game/SG_LevelSave.SG_LevelSave_C|GetPlayerTransform (Variables|Default|GetLevelSave))) "0, 0, 0")) ; If player transform not 0, move to there
      (Transformation|SetWorldTransform (Variables|/Script/Engine.Character|GetCapsuleComponent (Game|GetPlayerCharacter 0)) (Variables|/Game/SG_LevelSave.SG_LevelSave_C|GetPlayerTransform (Variables|Default|GetLevelSave)) false false))
    (else
      (bind _returnvalue_4 (SaveGame|CreateSaveGameObject "/Game/SG_LevelSave.SG_LevelSave_C"))
      (Variables|Default|SetLevelSave _returnvalue_4))))

(fn ConstructionScript)