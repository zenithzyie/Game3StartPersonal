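; BP_PatrolRoute is a patrol route Blueprint that supplies successive locations along a spline's points.
; Each GetPatrolLocation call first advances PatrolIndex by Direction, then returns that spline point's position in local space, not world space.
; IncrementPatrolIndex flips Direction on reaching the point count and resets it to forward at zero, giving back-and-forth traversal without clamping the index.
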(event Custom|IncrementPatrolIndex
  (Variables|Default|SetPatrolIndex (+ (Variables|Default|GetPatrolIndex) (Variables|Default|GetDirection)))
  (if (>= (Variables|Default|GetPatrolIndex) (Spline|GetNumberOfSplinePoints (Variables|Default|GetSpline)))
    (Variables|Default|SetDirection (* (Variables|Default|GetDirection) -1))
    (elif (<= (Variables|Default|GetPatrolIndex) 0)
      (Variables|Default|SetDirection 1))))

(fn ConstructionScript)

(fn GetPatrolLocation
  (CallFunction|IncrementPatrolIndex)
  (return (Spline|GetLocationatSplinePoint (Variables|Default|GetSpline) (Variables|Default|GetPatrolIndex) "Local")))