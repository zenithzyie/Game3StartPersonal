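; Interactable dialogue actor that steps through lines from DT_Dialogue when the player presses E.
; An outer sphere shows a brief "Press E" prompt, while another sphere enables input and creates the dialogue widget.
; Each press fills the text from the next row and sets material UV offsets on two images to match Speaker and Emotion.
; After the last row the widget is removed and the row index resets.
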(event OnComponentBeginOverlap(Sphere)
  (params (OverlappedComponent :type Primitive%20Component%20Object%20Reference) (OtherActor :type Actor%20Object%20Reference) (OtherComp :type Primitive%20Component%20Object%20Reference) (OtherBodyIndex :type Integer) (bFromSweep :type Boolean) (SweepResult :type Hit%20Result%20Structure%20%28by%20ref%29))
  ;[1 1 1] Add dialogue text to viewport
  (Utilities|Casting|CastToBP_ThirdPersonCharacter OtherActor)
  (Input|EnableInput (Game|GetPlayerController 0))
  (bind _returnvalue (UserInterface|CreateWidget "/Game/WidgetsUI/W_DataTableDialogue.W_DataTableDialogue_C"))
  (bind _output_get (Variables|Default|SetW_DataDialogue _returnvalue)))

(event OnComponentEndOverlap(Sphere)
  (params (OverlappedComponent :type Primitive%20Component%20Object%20Reference) (OtherActor :type Actor%20Object%20Reference) (OtherComp :type Primitive%20Component%20Object%20Reference) (OtherBodyIndex :type Integer))
  ;[1 1 1] Add dialogue text to viewport
  (Utilities|Casting|CastToBP_ThirdPersonCharacter OtherActor)
  (Widget|RemovefromParent (stale OnComponentBeginOverlap(Sphere) _output_get)))

(event OnComponentBeginOverlap(E_Sphere)
  (params (OverlappedComponent :type Primitive%20Component%20Object%20Reference) (OtherActor :type Actor%20Object%20Reference) (OtherComp :type Primitive%20Component%20Object%20Reference) (OtherBodyIndex :type Integer) (bFromSweep :type Boolean) (SweepResult :type Hit%20Result%20Structure%20%28by%20ref%29))
  ;[1 1 1] Press E to interact text overlap
  (if (== OtherActor (Game|GetPlayerCharacter 0))
    (bind _returnvalue (UserInterface|CreateWidget "/Game/WidgetsUI/W_PressE.W_PressE_C"))
    (bind _output_get (Variables|Default|SetCreateE _returnvalue))
    (UserInterface|Viewport|AddtoViewport _output_get 0)
    (Utilities|FlowControl|Delay 3.0)
    (Widget|RemovefromParent (Variables|Default|GetCreateE))))

(event OnComponentEndOverlap(E_Sphere)
  (params (OverlappedComponent :type Primitive%20Component%20Object%20Reference) (OtherActor :type Actor%20Object%20Reference) (OtherComp :type Primitive%20Component%20Object%20Reference) (OtherBodyIndex :type Integer))
  ;[1 1 1] Press E to interact text overlap
  (if (== (Game|GetPlayerCharacter 0) OtherActor)
    (Widget|RemovefromParent (Variables|Default|GetCreateE))))

(event Custom|NextLine
  (bind _w_datadialogue (Variables|Default|GetW_DataDialogue))
  (bind _image_0 (Variables|/Game/WidgetsUI/W_DataTableDialogue.W_DataTableDialogue_C|GetImage_0 _w_datadialogue))
  (bind _image_1 (Variables|/Game/WidgetsUI/W_DataTableDialogue.W_DataTableDialogue_C|GetImage_1 _w_datadialogue))
  (Utilities|FlowControl|Sequence
    (:then_0
      (Utilities|FlowControl|DoOnce false
        (:Completed
          (UserInterface|Viewport|AddtoViewport (Variables|Default|GetW_DataDialogue) 0)
          (UserInterface|Viewport|AddtoViewport (Variables|Default|GetCreateE) 0))))
    (:then_1
      (bind _outrownames (DataTable|GetDataTableRowNames "/Game/DataTables/DT_Dialogue.DT_Dialogue"))
      (if (< (Variables|Default|GetRowIndex) (Utilities|Array|Length _outrownames))
        (bind _returnvalue (Utilities|GetDataTableRow "/Game/DataTables/DT_Dialogue.DT_Dialogue" (Utilities|Array|Get(acopy) _outrownames (Variables|Default|GetRowIndex)))
          (:then
            (Rendering|Components|TextRender|SetText (Variables|/Game/WidgetsUI/W_DataTableDialogue.W_DataTableDialogue_C|GetDialText _w_datadialogue) (.text _returnvalue))
            (bind _returnvalue_2 (Appearance|GetDynamicMaterial _image_0 :!class /Script/UMG.Image))
            (Class|Image|SetBrushfromMaterial _image_0 _returnvalue_2)
            (Rendering|Material|SetVectorParameterValue _returnvalue_2 "UV Location" (Utilities|Struct|MakeLinearColor (.x (Utilities|Select :Index (.speaker _returnvalue) :NewEnumerator0 "5.000000,6.000000,0.000000" :NewEnumerator1 "5.000000,4.000000,0.000000")) (.y (Utilities|Select :Index (.speaker _returnvalue) :NewEnumerator0 "5.000000,6.000000,0.000000" :NewEnumerator1 "5.000000,4.000000,0.000000")) 0.0 1.0) :!class /Script/Engine.MaterialInstanceDynamic)
            (bind _returnvalue_3 (Appearance|GetDynamicMaterial _image_1 :!class /Script/UMG.Image))
            (Class|Image|SetBrushfromMaterial _image_1 _returnvalue_3)
            (Rendering|Material|SetVectorParameterValue _returnvalue_3 "UV Location" (Utilities|Struct|MakeLinearColor (.x (Utilities|Select :Index (.emotion _returnvalue) :NewEnumerator0 "0, 0, 0" :NewEnumerator1 "1.000000,2.000000,0.000000" :NewEnumerator2 "3.000000,1.000000,0.000000" :NewEnumerator3 "5.000000,2.000000,0.000000" :NewEnumerator4 "4.000000,0.000000,0.000000" :NewEnumerator5 "5.000000,6.000000,0.000000" :NewEnumerator6 "3.000000,1.000000,0.000000")) (.y (Utilities|Select :Index (.emotion _returnvalue) :NewEnumerator0 "0, 0, 0" :NewEnumerator1 "1.000000,2.000000,0.000000" :NewEnumerator2 "3.000000,1.000000,0.000000" :NewEnumerator3 "5.000000,2.000000,0.000000" :NewEnumerator4 "4.000000,0.000000,0.000000" :NewEnumerator5 "5.000000,6.000000,0.000000" :NewEnumerator6 "3.000000,1.000000,0.000000")) 0.0 1.0) :!class /Script/Engine.MaterialInstanceDynamic)
            (Math|Integer|IncrementInt (Variables|Default|GetRowIndex)))
          (:RowNotFound
            (Development|PrintString "no rows!!!")))
        (else
          (Widget|RemovefromParent (Variables|Default|GetW_DataDialogue))
          (Variables|Default|SetRowIndex 0))))))

(event Collision|EventActorBeginOverlap
  (params (OtherActor :type Actor%20Object%20Reference)))

(event EventTick
  (params (DeltaSeconds :type Float%20%28single-precision%29)))

(event Input|KeyboardEvents|E
  (params (Key :type Key%20Structure :default "None"))
  ;[1 1 1] Add dialogue text to viewport
  (:Pressed
    (CallFunction|NextLine)))

(fn ConstructionScript)