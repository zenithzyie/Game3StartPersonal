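; Debug actor that simulates bullet drop from an Arrow component and draws the predicted trajectory.
; Every 1.5 seconds it runs Unreal's built-in projectile path prediction alongside a hand-written BDC event.
; BDC steps line traces along the path, lowering Z velocity by a gravity term scaled by SimFrequency, until a hit or the step limit.
; It draws debug lines and spheres, prints each result, then resets to the arrow and starting velocity.
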(event Custom|BDC
  (Variables|Default|SetEnd (+ (Variables|Default|GetLine%20Start) (/ (Variables|Default|GetVelocity) (Math|Vector|MakeVector (Variables|Default|GetSimFrequency) 1.0 1.0))))
  (Utilities|FlowControl|ForLoopwithBreak 1 (Math|Float|Truncate (Variables|Default|GetSimFrequency)) :!label _label
    (:LoopBody
      (Rendering|Debug|DrawDebugLine (Variables|Default|GetLine%20Start) (Variables|Default|GetEnd) "(R=0.230611,G=0.178226,B=1.000000,A=1.000000)" (Variables|Default|GetMaxSimTime) 0.0)
      (Rendering|Debug|DrawDebugSphere (Variables|Default|GetEnd) 5.0 12 "(R=1.000000,G=0.140404,B=0.027083,A=1.000000)" (Variables|Default|GetMaxSimTime))
      (bind _returnvalue (Class|KismetSystemLibrary|LineTraceSinglebyProfile (Variables|Default|GetLine%20Start) (Variables|Default|GetEnd) "BlockAll" false 0 "ForDuration" true))
      (if _returnvalue
        (Development|PrintString "HIT SOMETHING")
        (goto _label Break)
        (else
          (Development|PrintString "DIDNT HIT")
          (Variables|Default|SetLine%20Start (Variables|Default|GetEnd))
          ;[1 1 1] Comment
          (Variables|Default|SetVelocity (+ (Variables|Default|GetVelocity) (Math|Vector|MakeVector 0.0 0.0 (/ -9.8e+02 (Math|Float|Square (Variables|Default|GetSimFrequency))))))
          ;[1 1 1] Comment
          (Variables|Default|SetEnd (+ (Variables|Default|GetLine%20Start) (/ (Variables|Default|GetVelocity) (Math|Vector|MakeVector (Variables|Default|GetSimFrequency) 1.0 1.0)))))))
    (:Completed
      ;[1 1 1] Comment
      (Variables|Default|SetLine%20Start (Transformation|GetWorldLocation (Variables|Default|GetArrow)))
      (Variables|Default|SetVelocity (Variables|Default|GetStartingVelocity)))))

(event EventBeginPlay
  (Variables|Default|SetEnd (+ (Variables|Default|GetLine%20Start) (/ (Variables|Default|GetVelocity) (Math|Vector|MakeVector (Variables|Default|GetSimFrequency) 1.0 1.0))))
  (Variables|Default|SetStartLocation (Transformation|GetWorldLocation (Variables|Default|GetArrow)))
  (Utilities|FlowControl|Sequence :!label _label
    (:then_0
      (Class|GameplayStatics|BlueprintPredictProjectilePathAdvanced (Utilities|Struct|MakePredictProjectilePathParams (Variables|Default|GetStartLocation) (Variables|Default|GetStartingVelocity) true 0.0 (Variables|Default|GetMaxSimTime) true "ECC_Pawn" "ObjectTypeQuery1" 0 (Variables|Default|GetSimFrequency) 0.0 "ForDuration" 1e+02 false))
      (Utilities|FlowControl|Delay 1.5)
      (goto _label))
    (:then_1
      (CallFunction|BDC))))

(fn ConstructionScript)