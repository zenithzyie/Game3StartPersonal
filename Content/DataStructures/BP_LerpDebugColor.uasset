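; Debug actor that visualizes HSV color interpolation with a vertical column of debug spheres.
; On BeginPlay, a 100-pass loop raises a Step value, which drives both sphere height above the actor and the blue-to-red HSV lerp alpha.
; Step grows by 0.1 per pass without clamping, so alpha runs well past 1.
; An unconnected Timeline branch holds a linear color lerp variant that never runs.
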(event EventBeginPlay
  (bind _returnvalue (Transformation|GetActorLocation))
  (for _index (range 0 99)
    (Rendering|Debug|DrawDebugSphere (Math|Vector|MakeVector (.x _returnvalue) (.y _returnvalue) (+ (.z _returnvalue) (* (Variables|Default|GetStep) 1.5e+03))) 1e+02 12 (Class|KismetMathLibrary|LinearColorLerpUsingHSV "(R=0.000000,G=0.161622,B=1.000000,A=1.000000)" "(R=1.000000,G=0.096325,B=0.000000,A=1.000000)" (Variables|Default|GetStep)) 12.0 4.0)
    (Variables|Default|SetStep (+ 0.1 (Variables|Default|GetStep)))))

(fn ConstructionScript)